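; Driveable BuggyTek vehicle Blueprint that adds horn, throttle and light controls on top of its parent class.
; While the clutch is disengaged, MoveForward sets throttle and uses input sign and current gear to drive brake and reverse lights.
; Reload or gamepad Special Left switches the headlight between visibility and beam-intensity states.
; RunOnServer, called on each axis update and headlight press, syncs emissive material parameters on DMI to headlight state.
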(event `Key|RightMouseButton`
  (:`Pressed`
    (`self.StartHonk`))
  (:`Released`
    (`self.StopHonk`)))

(event `InputAxis|MoveForward`
  (params (AxisValue :type "Float (single-precision)"))
  (bind _vehiclemovement (`self.VehicleMovement`))
  (bind _dmi (`self.DMI`))
  (bind _brake_light_rear_right (`self.Brake_Light_Rear_Right`))
  (bind _returnvalue (`WheeledVehicleMovementComponent.GetCurrentGear` _vehiclemovement))
  (bind _returnvalue_2 (== _returnvalue -1))
  (bind _returnvalue_3 (and _returnvalue_2 (> AxisValue 0.0)))
  (bind _returnvalue_4 (and (< AxisValue 0.0) (>= _returnvalue 0)))
  ;[1 1 1] Brake Light Conditions
  (`self.RunOnServer`)
  (if (not (`self.Clutch Engaged`))
    (`|ExecutionSequence`
      (:`then_0`
        (`WheeledVehicleMovementComponent.SetThrottleInput` _vehiclemovement AxisValue))
      (:`then_1`
        (if _returnvalue_4
          (`SceneComponent.SetVisibility` _brake_light_rear_right true true)
          (else
            (`SceneComponent.SetVisibility` _brake_light_rear_right _returnvalue_3 true)
            (`SceneComponent.SetVisibility` (`self.Reverse Light Righ`) _returnvalue_2 true))))
      (:`then_2`
        (if _returnvalue_4
          (`MaterialInstanceDynamic.SetScalarParameterValue` _dmi "Brake stop light power" 10.0 :!label _label)
          (`MaterialInstanceDynamic.SetVectorParameterValue` _dmi "Brake light color" (struct :`R` 0.33 :`G` 0.026033 :`B` 0.02 :`A` 1.0))
          (else
            (`MaterialInstanceDynamic.SetScalarParameterValue` _dmi "Brake stop light power" 0.1)
            (`MaterialInstanceDynamic.SetVectorParameterValue` _dmi "Brake light color" (struct :`R` 0.637 :`G` 0.05 :`B` 0.038 :`A` 1.0)))))
      (:`then_3`
        (if _returnvalue_3
          (goto _label))))))

(event `InputAction|Reload`
  (bind _headlight_right_parent (`self.Headlight_Right_Parent`))
  (:`Pressed`
    (`self.RunOnServer` :!label _label_2)
    (if (`SceneComponent.IsVisible` (`self.Headlight_Right_Parent`))
      (`SceneComponent.SetVisibility` _headlight_right_parent false true)
      (elif (`self.Are Lights on Low Beam`)
        (`LightComponent.SetIntensity` _headlight_right_parent (`self.Headlight Hight Beam`))
        (else
          (`SceneComponent.SetVisibility` _headlight_right_parent true true)
          (`LightComponent.SetIntensity` _headlight_right_parent (`self.Headlight Low Beam`)))))))

(event `Key|Gamepad_Special_Left`
  (:`Pressed`
    (goto _label_2)))

(event `RunOnServer`
  (bind _dmi (`self.DMI`))
  (bind _dmi_2 (`self.DMI`))
  (bind _dmi_3 (`self.DMI`))
  (bind _dmi_4 (`self.DMI`))
  (`|ExecutionSequence`
    (:`then_0`
      (if (`SceneComponent.IsVisible` (`self.Headlight_Right_Parent`))
        (`MaterialInstanceDynamic.SetScalarParameterValue` _dmi "Headlight power" 10.0 :!label _label_3)
        (`MaterialInstanceDynamic.SetVectorParameterValue` _dmi "Headlight color" (struct :`R` 1.0 :`G` 0.774227 :`B` 0.447871 :`A` 1.0))
        (elif (`self.Are Lights on Low Beam`)
          (goto _label_3)
          (else
            (`MaterialInstanceDynamic.SetScalarParameterValue` _dmi_2 "Headlight power" 0.1)
            (`MaterialInstanceDynamic.SetVectorParameterValue` _dmi_2 "Headlight color" (struct :`R` 1.0 :`G` 0.774227 :`B` 0.447871 :`A` 1.0))))))
    (:`then_1`
      (if (`SceneComponent.IsVisible` (`self.Headlight_Right_Parent`))
        (`MaterialInstanceDynamic.SetScalarParameterValue` _dmi_4 "Brake light power" 10.0 :!label _label_4)
        (`MaterialInstanceDynamic.SetVectorParameterValue` _dmi_4 "Brake light color" (struct :`R` 0.373615 :`G` 0.001202 :`B` 0.000638 :`A` 1.0))
        (elif (`self.Are Lights on Low Beam`)
          (goto _label_4)
          (else
            (`MaterialInstanceDynamic.SetScalarParameterValue` _dmi_3 "Brake light power" 0.1)
            (`MaterialInstanceDynamic.SetVectorParameterValue` _dmi_3 "Brake light color" (struct :`R` 0.373615 :`G` 0.001202 :`B` 0.000638 :`A` 1.0))))))))

(event `self.ReceiveBeginPlay`
  (bind _returnvalue (`self.GetOwnerController`))
  (`self.EnableInput` _returnvalue))

(fn `UserConstructionScript`
  (`parent.UserConstructionScript`))